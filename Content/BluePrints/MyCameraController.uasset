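; Camera controller for viewing a Model actor, which adds a MyWidgetBlueprint UI to the viewport on BeginPlay.
; Horizontal touch drags yaw the model, and Tick spins it steadily while AutoRotateMode is on.
; Gamepad sticks translate the camera actor along its own axes, and custom events set the FOV and auto-rotate mode.
; Look-at, two-finger distance and axis-driven yaw logic is present but unwired, so it never runs.
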(event `InputTouch`
  (params (Location :type "Vector Structure") (FingerIndex :type "ETouchIndex Enum"))
  (:`Pressed`
    (set `self.TouchStart` Location))
  (:`Moved`
    (`self.K2_AddActorWorldRotation` (`self.Model`) (`KismetMathLibrary.MakeRotator` 0.0 0.0 (* (* 5 (.x (- (`self.TouchStart`) Location))) (`GameplayStatics.GetWorldDeltaSeconds`))) false false)
    (set `self.TouchStart` Location)))

(event `SetFOV`
  (params (fov :type "Float (double-precision)"))
  ;[1 1 1] Set FOV
  (`CameraComponent.SetFieldOfView` (`self.Camera`) fov))

(event `InputAxisKey|Gamepad_LeftX`
  (params (AxisValue :type "Float (single-precision)"))
  ;[1 1 1] 移动控制
  (`self.K2_AddActorWorldOffset` (* (`self.GetActorRightVector`) (`self.GetInputAxisKeyValue`))))

(event `InputAxisKey|Gamepad_LeftY`
  (params (AxisValue :type "Float (single-precision)"))
  ;[1 1 1] 移动控制
  (`self.K2_AddActorWorldOffset` (* (`self.GetActorForwardVector`) (`self.GetInputAxisKeyValue`))))

(event `self.ReceiveBeginPlay`
  (bind _returnvalue (`|CreateWidget` "/Game/BluePrints/MyWidgetBlueprint.MyWidgetBlueprint_C"))
  (`UserWidget.AddToViewport` _returnvalue 0))

(event `ChangeAutoRotate`
  (params (mode :type Boolean))
  (set `self.AutoRotateMode` mode))

(event `self.ReceiveTick`
  (params (DeltaSeconds :type "Float (single-precision)"))
  (bind _model (`self.Model`))
  (if (`self.AutoRotateMode`)
    (if (`KismetSystemLibrary.IsValid` _model)
      (`self.K2_AddActorWorldRotation` _model (`KismetMathLibrary.MakeRotator` 0.0 0.0 (* -10 DeltaSeconds)) false false))))

(event `InputAxisKey|Gamepad_RightX`
  (params (AxisValue :type "Float (single-precision)"))
  ;[1 1 1] 摄像机视角控制
  (`self.K2_AddActorWorldOffset` (* (`self.GetActorRightVector`) (`self.GetInputAxisKeyValue`))))

(event `InputAxisKey|Gamepad_RightY`
  (params (AxisValue :type "Float (single-precision)"))
  ;[1 1 1] 摄像机视角控制
  (`self.K2_AddActorWorldOffset` (* (`self.GetActorUpVector`) AxisValue)))

(fn `UserConstructionScript`)